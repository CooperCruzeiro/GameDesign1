(event OnComponentBeginOverlap(Sphere)
  (params (OverlappedComponent :type Primitive%20Component%20Object%20Reference) (OtherActor :type Actor%20Object%20Reference) (OtherComp :type Primitive%20Component%20Object%20Reference) (OtherBodyIndex :type Integer) (bFromSweep :type Boolean) (SweepResult :type Hit%20Result%20Structure%20%28by%20ref%29))
  (bind _asbp_third_person_game_mode_custom (Utilities|Casting|CastToBP_ThirdPersonGameModeCustom (Game|GetGameMode)))
  (if (not (stale _output_get))
    (bind _output_get (Variables|/Game/Blueprints/BP_ThirdPersonGameModeCustom.BP_ThirdPersonGameModeCustom_C|SetisGameOver _asbp_third_person_game_mode_custom true))
    (Actor|DestroyActor)
    (bind _returnvalue (UserInterface|CreateWidget "/Game/Widgets/W_YouWin.W_YouWin_C"))
    (UserInterface|Viewport|AddtoViewport _returnvalue 0)))

(event OnComponentBeginOverlap(SumoStatue)
  (params (OverlappedComponent :type Primitive%20Component%20Object%20Reference) (OtherActor :type Actor%20Object%20Reference) (OtherComp :type Primitive%20Component%20Object%20Reference) (OtherBodyIndex :type Integer) (bFromSweep :type Boolean) (SweepResult :type Hit%20Result%20Structure%20%28by%20ref%29)))

(event EventBeginPlay
  (bind _newtrack_0 (Timeline|Spin%20Finish Play)
    (:Update
      (Transformation|SetActorRelativeRotation (Math|Rotator|MakeRotator 0.0 0.0 (* _newtrack_0 3.6e+02))))))

(event EventTick
  (params (DeltaSeconds :type Float%20%28single-precision%29)))

(fn ConstructionScript)