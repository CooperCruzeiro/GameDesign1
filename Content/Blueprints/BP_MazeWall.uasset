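; BP_MazeWall is a maze wall actor that slides horizontally to a new position shortly after play begins.
; BeginPlay stores the start location, waits briefly, then runs the MoveWall timeline to lerp the actor, unswept, toward an offset given by Movement scaled on X and Y.
; The wall sound is triggered on every timeline update, so it restarts repeatedly during the move rather than playing once.
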(event EventBeginPlay
  (Variables|Default|SetStart (Transformation|GetActorLocation))
  (Utilities|FlowControl|Delay 2.0)
  (bind _move_wall (Timeline|Move%20Wall Play)
    (:Update
      (Audio|PlaySoundatLocation "/Game/Audio/Cue_MazeWalls.Cue_MazeWalls" (Transformation|GetWorldLocation (Variables|Default|GetDefaultSceneRoot)) "0, 0, 0" 1.0 1.0 0.0 "/Game/Audio/A_MazeWalls.A_MazeWalls" 0 0 0)
      (Transformation|SetActorLocation (Math|Vector|Lerp(Vector) (Variables|Default|GetStart) (+ (Variables|Default|GetStart) (* (Variables|Default|GetMovement) "166.700000,166.700000,0.000000")) _move_wall) false false))))

(event Collision|EventActorBeginOverlap
  (params (OtherActor :type Actor%20Object%20Reference)))

(event EventTick
  (params (DeltaSeconds :type Float%20%28single-precision%29)))

(fn ConstructionScript)