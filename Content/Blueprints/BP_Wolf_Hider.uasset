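; BP_Wolf_Hider is a trigger-driven moving wall that leads into the death screen.
; Overlapping its Box plays the LiftWall timeline, which moves the Cube along relative Z.
; The timeline's Update pin also feeds a delayed chain that plays a scream, shows W_EndScreen, then W_YouDied after another delay.
; StartLocation is stored at BeginPlay but never used.
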(event OnComponentBeginOverlap(Box)
  (params (OverlappedComponent :type Primitive%20Component%20Object%20Reference) (OtherActor :type Actor%20Object%20Reference) (OtherComp :type Primitive%20Component%20Object%20Reference) (OtherBodyIndex :type Integer) (bFromSweep :type Boolean) (SweepResult :type Hit%20Result%20Structure%20%28by%20ref%29))
  (Development|PrintString "Moving Wall" true true "(R=0.000000,G=1.000000,B=0.409326,A=1.000000)")
  (bind _liftwall (Timeline|Lift%20Wall Play)
    (:Update
      (Transformation|SetRelativeLocation (Variables|Default|GetCube) (Math|Vector|MakeVector 0.0 0.0 (* _liftwall 1e+03)) false false)
      (Utilities|FlowControl|Delay 4.0)
      (Audio|PlaySoundatLocation "/Game/Audio/man-scream-121085.man-scream-121085" (Transformation|GetActorLocation) "0, 0, 0" 1.0 1.0 0.0 0 0 0 0)
      (bind _returnvalue (UserInterface|CreateWidget "/Game/Widgets/W_EndScreen.W_EndScreen_C"))
      (UserInterface|Viewport|AddtoViewport _returnvalue 0)
      (Utilities|FlowControl|Delay 1.0)
      (bind _returnvalue_2 (UserInterface|CreateWidget "/Game/Widgets/W_YouDied.W_YouDied_C"))
      (UserInterface|Viewport|AddtoViewport _returnvalue_2 0))))

(event EventBeginPlay
  (Variables|Default|SetStart%20Location (Transformation|GetActorLocation)))

(event Collision|EventActorBeginOverlap
  (params (OtherActor :type Actor%20Object%20Reference)))

(event EventTick
  (params (DeltaSeconds :type Float%20%28single-precision%29)))

(fn ConstructionScript)