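; BP_ProjectileSpawn is a spawner actor that repeatedly launches soccer balls at the player.
; Once triggered, its SpawnProjectile event spawns a BP_SoccerBall_Projectile at its own transform, pauses briefly, then applies a strong impulse to the ball mesh toward player character 0's current location.
; After a longer delay the event loops back to spawn again, with no exit condition.
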(event Custom|SpawnProjectile
  (bind _returnvalue (Game|SpawnActorfromClass "/Game/Blueprints/Soccer/BP_SoccerBall_Projectile.BP_SoccerBall_Projectile_C" (Transformation|GetActorTransform) "Undefined" "MultiplyWithRoot" 0 0 :!label _label))
  (Utilities|FlowControl|Delay 0.6)
  (Physics|AddImpulse (Variables|/Game/Blueprints/Soccer/BP_SoccerBall_Projectile.BP_SoccerBall_Projectile_C|GetBallMesh _returnvalue) (* (Math|Vector|Normalize (- (Transformation|GetActorLocation (Game|GetPlayerCharacter 0)) (Transformation|GetActorLocation))) "100000.000000,100000.000000,100000.000000") "None" false)
  (Utilities|FlowControl|Delay 5.0)
  (goto _label))

(event EventBeginPlay)

(fn ConstructionScript)