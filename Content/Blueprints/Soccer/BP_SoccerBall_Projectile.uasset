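; Soccer ball projectile that knocks the player into ragdoll when it hits a character fast enough.
; On a mesh hit with a custom third-person character, it checks ball speed, then ragdolls player 0 rather than the hit actor.
; It applies an impulse at the hit bone along the impact normal, scaled by ball speed, character mesh mass and a tuning factor.
; Speed-based switching between capsule and mesh collision is disconnected, and debug prints remain.
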(event OnComponentHit(BallMesh)
  (params (HitComponent :type Primitive%20Component%20Object%20Reference) (OtherActor :type Actor%20Object%20Reference) (OtherComp :type Primitive%20Component%20Object%20Reference) (NormalImpulse :type Vector :default "0, 0, 0") (Hit :type Hit%20Result%20Structure%20%28by%20ref%29))
  (bind (_bblockinghit _binitialoverlap _time _distance _location _impactpoint _normal _impactnormal _physmat _hitactor _hitcomponent _hitbonename) (Collision|BreakHitResult Hit))
  (Utilities|Casting|CastToBP_ThirdPersonCharacterCustom OtherActor)
  ;[1 1 1] Is Ball's speed fast enough to affect player
  (if (>= (Math|Vector|VectorLength (Transformation|GetVelocity)) 8e+02)
    (Development|PrintString "Hello")
    (bind _asbp_third_person_character_custom (Utilities|Casting|CastToBP_ThirdPersonCharacterCustom (Game|GetPlayerCharacter 0)))
    (Default|RagdollMode _asbp_third_person_character_custom)
    (Development|PrintString (Utilities|String|ToString(Vector) (* _impactnormal (* (Math|Vector|VectorLength (Transformation|GetVelocity)) (Physics|GetMass (Variables|/Script/Engine.Character|GetMesh _asbp_third_person_character_custom)) (Variables|Default|GetImpulseScalingFactor)))))
    (Default|ApplyBallForce _asbp_third_person_character_custom _impactpoint (* _impactnormal (* (Math|Vector|VectorLength (Transformation|GetVelocity)) (Physics|GetMass (Variables|/Script/Engine.Character|GetMesh _asbp_third_person_character_custom)) (Variables|Default|GetImpulseScalingFactor))) _hitbonename)))

(event EventBeginPlay)

(event Collision|EventActorBeginOverlap
  (params (OtherActor :type Actor%20Object%20Reference)))

(event EventTick
  (params (DeltaSeconds :type Float%20%28single-precision%29))
  ;[1 1 1] If ball is fast enough, change collision from capsule to mesh, so that the ball bounces off the player more realistically at high speeds. If not, reset to using capsule collision
)

(fn ConstructionScript)