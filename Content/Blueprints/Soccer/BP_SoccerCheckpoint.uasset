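; BP_SoccerCheckpoint is a cone checkpoint that counts a BP_SoccerBall passing through its box trigger, once per checkpoint.
; The first ball overlap increments TotalConesPassed on the referenced door and prints a debug message.
; When that count reaches TotalConeCount, it loops over all BP_SoccerDoor actors but calls AllConesPassed only on DoorReference, once per iteration, if its DoorID is 1.
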(event OnComponentBeginOverlap(Box)
  (params (OverlappedComponent :type Primitive%20Component%20Object%20Reference) (OtherActor :type Actor%20Object%20Reference) (OtherComp :type Primitive%20Component%20Object%20Reference) (OtherBodyIndex :type Integer) (bFromSweep :type Boolean) (SweepResult :type Hit%20Result%20Structure%20%28by%20ref%29))
  (bind _doorreference (Variables|Default|GetDoorReference))
  (bind _doorreference_2 (Variables|Default|GetDoorReference))
  (Utilities|Casting|CastToBP_SoccerBall OtherActor)
  (if (not (Variables|Default|GetBeenPassed))
    (bind _result (Math|Integer|IncrementInt (Variables|/Game/Blueprints/Soccer/BP_SoccerDoor.BP_SoccerDoor_C|GetTotalConesPassed _doorreference_2))
      (:%20%20
        (Variables|/Game/Blueprints/Soccer/BP_SoccerDoor.BP_SoccerDoor_C|SetTotalConesPassed _doorreference_2 _result)
        (Development|PrintString "Cone Passed" true true "(R=1.000000,G=0.257831,B=0.000000,A=1.000000)")
        (Variables|Default|SetBeenPassed true)
        (if (>= (Variables|/Game/Blueprints/Soccer/BP_SoccerDoor.BP_SoccerDoor_C|GetTotalConesPassed _doorreference_2) (Variables|/Game/Blueprints/Soccer/BP_SoccerDoor.BP_SoccerDoor_C|GetTotalConeCount _doorreference_2))
          (bind _outactors (Actor|GetAllActorsOfClass "/Game/Blueprints/Soccer/BP_SoccerDoor.BP_SoccerDoor_C"))
          (for _array_element _outactors
            (Utilities|IsValid _doorreference
              (:Is%20Valid
                (if (== (Variables|/Game/Blueprints/Soccer/BP_SoccerDoor.BP_SoccerDoor_C|GetDoorID _doorreference) 1)
                  (Default|AllConesPassed _doorreference))))))))))

(event EventBeginPlay)

(event Collision|EventActorBeginOverlap
  (params (OtherActor :type Actor%20Object%20Reference)))

(event EventTick
  (params (DeltaSeconds :type Float%20%28single-precision%29)))

(fn ConstructionScript)