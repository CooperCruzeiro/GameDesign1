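; BP_SoccerTarget is a one-shot soccer target that counts toward opening a linked BP_SoccerDoor.
; The first BP_SoccerBall hit on its cylinder enables physics, applies an impulse along the impact normal and increments the door's hit count.
; At the required total, it loops over all doors but tests only its linked one: if DoorID is 2, it calls AllTargetsHit and destroys every target after a delay.
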(event OnComponentHit(Cylinder)
  (params (HitComponent :type Primitive%20Component%20Object%20Reference) (OtherActor :type Actor%20Object%20Reference) (OtherComp :type Primitive%20Component%20Object%20Reference) (NormalImpulse :type Vector :default "0, 0, 0") (Hit :type Hit%20Result%20Structure%20%28by%20ref%29))
  (bind _doorreference (Variables|Default|GetDoorReference))
  (bind _doorreference_2 (Variables|Default|GetDoorReference))
  (Utilities|Casting|CastToBP_SoccerBall OtherActor)
  (if (not (Variables|Default|GetBeenHit))
    (Physics|SetSimulatePhysics (Variables|Default|GetCylinder) true)
    (Physics|AddImpulse (Variables|Default|GetCylinder) (.impactnormal Hit) "None" false)
    (Development|PrintString "Hit Target" true true "(R=0.009953,G=0.000000,B=1.000000,A=1.000000)")
    (bind _result (Math|Integer|IncrementInt (Variables|/Game/Blueprints/Soccer/BP_SoccerDoor.BP_SoccerDoor_C|GetTotalTargetsHit _doorreference_2))
      (:%20%20
        (Variables|/Game/Blueprints/Soccer/BP_SoccerDoor.BP_SoccerDoor_C|SetTotalTargetsHit _doorreference_2 _result)
        (Variables|Default|SetBeenHit true)
        (if (>= (Variables|/Game/Blueprints/Soccer/BP_SoccerDoor.BP_SoccerDoor_C|GetTotalTargetsHit _doorreference_2) (Variables|/Game/Blueprints/Soccer/BP_SoccerDoor.BP_SoccerDoor_C|GetTotalTargets _doorreference_2))
          (bind _outactors (Actor|GetAllActorsOfClass "/Game/Blueprints/Soccer/BP_SoccerDoor.BP_SoccerDoor_C"))
          (for _array_element _outactors
            (Utilities|IsValid _doorreference
              (:Is%20Valid
                (if (== (Variables|/Game/Blueprints/Soccer/BP_SoccerDoor.BP_SoccerDoor_C|GetDoorID _doorreference) 2)
                  (Default|AllTargetsHit _doorreference)
                  (bind _outactors_2 (Actor|GetAllActorsOfClass "BP_SoccerTarget_C"))
                  (Utilities|FlowControl|Delay 3.0)
                  (Actor|DestroyActor _outactors_2))))))))))

(event OnComponentBeginOverlap(Cylinder)
  (params (OverlappedComponent :type Primitive%20Component%20Object%20Reference) (OtherActor :type Actor%20Object%20Reference) (OtherComp :type Primitive%20Component%20Object%20Reference) (OtherBodyIndex :type Integer) (bFromSweep :type Boolean) (SweepResult :type Hit%20Result%20Structure%20%28by%20ref%29)))

(event EventBeginPlay)

(event Collision|EventActorBeginOverlap
  (params (OtherActor :type Actor%20Object%20Reference)))

(event EventTick
  (params (DeltaSeconds :type Float%20%28single-precision%29)))

(fn ConstructionScript)